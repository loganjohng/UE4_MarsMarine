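; BP_MarsMarine_GameMode is the game mode that spawns alien enemies in waves.
; Shortly after BeginPlay it calls SetupNewWave, which increments CurrentWave and starts a looping timer by function name intended to drive alien spawning.
; SpawnAlien places a BP_Alien at a TargetPoint picked at random from all those in the level.
; Nothing here stops the timer or advances to a further wave.
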(event Custom|Spawn%20Wave
  (CallFunction|SpawnAlien))

(event EventBeginPlay
  (Utilities|FlowControl|Delay 2.0)
  (CallFunction|SetupNewWave))

(event EventTick
  (params (DeltaSeconds :type Float%20%28single-precision%29)))

(fn ConstructionScript)

(fn SetupNewWave
  (Math|Integer|IncrementInt (Variables|Default|GetCurrent%20Wave)
    (:%20%20
      (Utilities|Time|SetTimerbyFunctionName 0 "Spawn Wave" 1.0 true))))

(fn SpawnAlien
  (bind _spawn_point (CallFunction|GetRandomSpawnPoint))
  (Utilities|IsValid _spawn_point
    (:Is%20Valid
      (Game|SpawnActorfromClass "/Game/Blueprints/AI/BP_Alien.BP_Alien_C" (Transformation|GetActorTransform _spawn_point) "Undefined" 0 0))))

(fn GetRandomSpawnPoint
  (bind _outactors (Actor|GetAllActorsOfClass "/Script/Engine.TargetPoint"))
  (return (Utilities|Array|Get(acopy) _outactors (Math|Random|RandomIntegerinRange 0 (Utilities|Array|LastIndex _outactors)))))