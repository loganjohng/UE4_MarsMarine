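; Alien enemy character that chases the player marine and attacks in melee until it is killed.
; A retrying AI MoveTo loop drives the chase, while Tick checks range and pauses movement during the attack montage.
; DamagePlayer applies hit damage but is not called within this Blueprint.
; Incoming damage lowers health; at zero the alien disables movement and collision, increments the marine's kills and is destroyed after a delay.
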(event EventBeginPlay
  ;[1 1 1] AI follows the player
  (if (CallFunction|IsAlive) :!label _label
    (AI|AIMoveTo self "0, 0, 0" (Game|GetPlayerCharacter 0) 5.0 false
      (:OnSuccess
        _)
      (:OnFail
        _))
    (Utilities|FlowControl|Delay 0.2)
    (goto _label)))

(event Game|Damage|EventAnyDamage
  (params (Damage :type Float%20%28single-precision%29) (DamageType :type Damage%20Type%20Object%20Reference) (InstigatedBy :type Controller%20Object%20Reference) (DamageCauser :type Actor%20Object%20Reference))
  ;[1 1 1] When Alien takes damage
  (if (CallFunction|IsAlive)
    (CallFunction|DecreaseHealth Damage)
    (if (== (Variables|Default|GetHealth) 0.0)
      (CallFunction|KillAI)
      (Utilities|FlowControl|Delay 3.0)
      (Actor|DestroyActor))))

(event EventTick
  (params (DeltaSeconds :type Float%20%28single-precision%29))
  ;[1 1 1] When Alien attacks player
  (if (CallFunction|CanAttack)
    (CallFunction|DeactivateAIMovement)
    (Animation|Montage|PlayMontage (Variables|Character|GetMesh) "/Game/Characters/Enemy_Great_Spider/Animations/AlienAttack1.AlienAttack1"
      (:OnCompleted
        (if (CallFunction|IsAlive)
          (CallFunction|ActivateAIMovement))))))

(fn ConstructionScript)

(fn IsWithinAttackRange
  (bind _returnvalue (Game|GetPlayerCharacter 0))
  (bind _asbp_marine (Utilities|Casting|CastToBP_Marine _returnvalue))
  (if (Default|IsAlive _asbp_marine)
    (return (< (Transformation|GetDistanceTo _returnvalue) (Variables|Default|GetAttack%20Range)))))

(fn IsAttacking
  (return (Animation|Montage|MontageIsPlaying (Components|SkeletalMesh|GetAnimInstance (Variables|Character|GetMesh)) "/Game/Characters/Enemy_Great_Spider/Animations/AlienAttack1.AlienAttack1")))

(fn DeactivateAIMovement
  (Components|Movement|StopMovementImmediately (Variables|Character|GetCharacterMovement))
  (Components|Activation|Deactivate (Variables|Character|GetCharacterMovement)))

(fn ActivateAIMovement
  (Components|Activation|Activate (Variables|Character|GetCharacterMovement) false))

(fn DamagePlayer
  (if (CallFunction|IsAlive)
    (Game|Damage|ApplyDamage (Game|GetPlayerCharacter 0) (Variables|Default|GetDamage%20Per%20Hit) 0 0)))

(fn DecreaseHealth
  (params (Damage :type Float%20%28single-precision%29))
  (Variables|Default|SetHealth (Math|Float|Clamp(Float) (- (Variables|Default|GetHealth) Damage) 0.0 1e+02))
  (return 0.0))

(fn KillAI
  (Variables|Default|SetDead true)
  (CallFunction|DeactivateAIMovement)
  (Collision|SetActorEnableCollision false)
  (bind _asbp_marine (Utilities|Casting|CastToBP_Marine (Game|GetPlayerCharacter 0)))
  (Default|IncreaseKills _asbp_marine))

(fn IsAlive
  (return (not (Variables|Default|GetDead))))

(fn CanAttack
  (return (Math|Boolean|ANDBoolean (CallFunction|IsWithinAttackRange) (CallFunction|IsAlive) (not (CallFunction|IsAttacking)))))